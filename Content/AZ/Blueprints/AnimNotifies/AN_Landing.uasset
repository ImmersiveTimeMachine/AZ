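; Landing anim notify state for AZ_BP_Hero that refreshes movement state and adds forward momentum while active.
; Each tick it copies AZ_ABP_Hero's calculated movement state into the server and client state variables, identically on both authority branches.
; It then applies a velocity-change impulse along the last update velocity, scaled by a small random factor.
; Begin and End hold disconnected max walk speed override and restore logic, so both only return false.
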(fn ReceivedNotifyBegin
  (params (MeshComp :type Skeletal%20Mesh%20Component%20Object%20Reference) (Animation :type Anim%20Sequence%20Base%20Object%20Reference) (TotalDuration :type Float%20%28single-precision%29) (EventReference :type Anim%20Notify%20Event%20Reference%20Structure%20%28by%20ref%29))
  (return false))

(fn ReceivedNotifyTick
  (params (MeshComp :type Skeletal%20Mesh%20Component%20Object%20Reference) (Animation :type Anim%20Sequence%20Base%20Object%20Reference) (FrameDeltaTime :type Float%20%28single-precision%29) (EventReference :type Anim%20Notify%20Event%20Reference%20Structure%20%28by%20ref%29))
  (bind _asaz_abp_hero (Utilities|Casting|CastToAZ_ABP_Hero (Components|SkeletalMesh|GetAnimInstance MeshComp)))
  (bind _asaz_bp_hero (Utilities|Casting|CastToAZ_BP_Hero (Class|AnimInstance|GetOwningActor _asaz_abp_hero)))
  (bind _character_state (Default|CalculateMovementState _asaz_abp_hero))
  (if (Ability|HasAuthority _asaz_bp_hero)
    (bind _output_get (Variables|/Game/AZ/Blueprints/Animation/AZ_ABP_Hero.AZ_ABP_Hero_C|SetServer_CharacterState _asaz_abp_hero _character_state))
    (Variables|/Game/AZ/Blueprints/Animation/AZ_ABP_Hero.AZ_ABP_Hero_C|SetClient_CharacterState _asaz_abp_hero _output_get)
    (else
      (bind _output_get_2 (Variables|/Game/AZ/Blueprints/Animation/AZ_ABP_Hero.AZ_ABP_Hero_C|SetServer_CharacterState _asaz_abp_hero _character_state))
      (Variables|/Game/AZ/Blueprints/Animation/AZ_ABP_Hero.AZ_ABP_Hero_C|SetClient_CharacterState _asaz_abp_hero _output_get_2)))
  (Physics|AddImpulse (Variables|/Script/Engine.Character|GetCharacterMovement _asaz_bp_hero) (* (Pawn|Components|CharacterMovement|GetLastUpdateVelocity (Variables|/Script/Engine.Character|GetCharacterMovement _asaz_bp_hero)) (Math|Vector|Lerp(Vector) "0.010000,0.010000,0.010000" "0.050000,0.050000,0.050000" (Math|Random|RandomFloat))) true)
  (return true))

(fn ReceivedNotifyEnd
  (params (MeshComp :type Skeletal%20Mesh%20Component%20Object%20Reference) (Animation :type Anim%20Sequence%20Base%20Object%20Reference) (EventReference :type Anim%20Notify%20Event%20Reference%20Structure%20%28by%20ref%29))
  (return false))