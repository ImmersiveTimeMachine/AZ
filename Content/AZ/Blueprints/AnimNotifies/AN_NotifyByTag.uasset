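; Animation notify that sends a configurable gameplay event to the mesh's owner and edits gameplay tags on the hero.
; If the owner is an AZ_BP_Hero with a valid Ability System Component, it adds one tag set unless all are present.
; It then removes a second set only when the hero has every tag in it.
; Both edits use non-replicated loose tags.
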(fn ReceivedNotify
  (params (MeshComp :type Skeletal%20Mesh%20Component%20Object%20Reference) (Animation :type Anim%20Sequence%20Base%20Object%20Reference) (EventReference :type Anim%20Notify%20Event%20Reference%20Structure%20%28by%20ref%29))
  (bind _returnvalue (Components|GetOwner MeshComp))
  (bind _notifygameplaytagstoadd (Variables|Default|GetNotifyGameplayTagsToAdd))
  (bind _notifygameplaytagstoremove (Variables|Default|GetNotifyGameplayTagsToRemove))
  (Ability|SendGameplayEventtoActor _returnvalue (Variables|Default|GetNotifyEventTag))
  (bind _asaz_bp_hero (Utilities|Casting|CastToAZ_BP_Hero _returnvalue))
  (Utilities|IsValid (Class|AZCharacterBase|GetASC _asaz_bp_hero)
    (:Is%20Valid
      (if (GameplayTags|HasAllMatchingGameplayTags (Class|AZCharacterBase|GetASC _asaz_bp_hero) _notifygameplaytagstoadd)
        _
        (else
          (Ability|GameplayEffect|AddLooseGameplayTags _asaz_bp_hero _notifygameplaytagstoadd)))
      (if (GameplayTags|HasAllMatchingGameplayTags (Class|AZCharacterBase|GetASC _asaz_bp_hero) _notifygameplaytagstoremove)
        (Ability|GameplayEffect|RemoveLooseGameplayTags _asaz_bp_hero _notifygameplaytagstoremove))
      (return false))))