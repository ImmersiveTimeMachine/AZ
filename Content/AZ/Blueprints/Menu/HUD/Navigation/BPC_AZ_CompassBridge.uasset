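; Player controller component that bridges compass and world marker requests to the HUD compass module, acting only for the local controller that owns that module.
; Marker updates and show/hide calls forward once the module is attached and marked ready.
; Until then it queues markers in capped maps keyed by actor or scene component and stores visibility, which MarkReady replays.
; Removals clear queued entries and reach any valid module regardless of readiness.
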(event EventBeginPlay)

(event EventTick
  (params (DeltaSeconds :type Float%20%28single-precision%29)))

(event EventEndPlay
  (params (EndPlayReason :type EEndPlayReason%20Enum :default "Destroyed"))
  (Variables|Navigation|Bridge|SetbReady false)
  (Variables|Navigation|Bridge|SetbAttached false)
  (Utilities|Map|Clear (Variables|Navigation|Bridge|GetPendingCompass))
  (Utilities|Map|Clear (Variables|Navigation|Bridge|GetPendingWorld))
  (Variables|Navigation|Bridge|SetModuleRef 0)
  (Variables|Navigation|Bridge|SetbPendingVisibility false))

(fn AddorUpdateCompassMarker
  (params (Marker_Object :type Object%20Object%20Reference) (MarkerInfo :type S%20Compass%20Marker%20Info%20H%20Structure))
  (bind _moduleref (Variables|Navigation|Bridge|GetModuleRef))
  (bind _asplayer_controller (Utilities|Casting|CastToPlayerController (Components|GetOwner)))
  (if (Pawn|IsLocalController _asplayer_controller)
    (if (and (Utilities|IsValid Marker_Object) (or (Class|GameplayStatics|ObjectIsA Marker_Object "/Script/Engine.Actor") (Class|GameplayStatics|ObjectIsA Marker_Object "/Script/Engine.SceneComponent")))
      (if (and (Variables|Navigation|Bridge|GetbReady) (Utilities|IsValid (Variables|Navigation|Bridge|GetModuleRef)))
        (if (Utilities|IsValid _moduleref)
          (if (== (Widget|GetOwningPlayer _moduleref) _asplayer_controller)
            (Utilities|Map|Remove (Variables|Navigation|Bridge|GetPendingCompass) Marker_Object)
            (Default|AddorUpdateCompassMarker (Variables|Navigation|Bridge|GetModuleRef) Marker_Object MarkerInfo)))
        (elif (or (Utilities|Map|Contains (Variables|Navigation|Bridge|GetPendingCompass) Marker_Object) (< (Utilities|Map|Length (Variables|Navigation|Bridge|GetPendingCompass)) 128))
          (Utilities|Map|Add (Variables|Navigation|Bridge|GetPendingCompass) Marker_Object MarkerInfo)
          (else
            (Variables|Navigation|Bridge|SetbPendingOverflow true)))))))

(fn RemoveCompassMarker
  (params (Marker_Object :type Object%20Object%20Reference))
  (bind _moduleref (Variables|Navigation|Bridge|GetModuleRef))
  (bind _asplayer_controller (Utilities|Casting|CastToPlayerController (Components|GetOwner)))
  (if (Pawn|IsLocalController _asplayer_controller)
    (Utilities|Map|Remove (Variables|Navigation|Bridge|GetPendingCompass) Marker_Object)
    (if (Utilities|IsValid (Variables|Navigation|Bridge|GetModuleRef))
      (if (Utilities|IsValid _moduleref)
        (if (== (Widget|GetOwningPlayer _moduleref) _asplayer_controller)
          (Default|RemoveCompassMarker (Variables|Navigation|Bridge|GetModuleRef) Marker_Object))))))

(fn RemoveAllCompassMarkers
  (bind _moduleref (Variables|Navigation|Bridge|GetModuleRef))
  (bind _asplayer_controller (Utilities|Casting|CastToPlayerController (Components|GetOwner)))
  (if (Pawn|IsLocalController _asplayer_controller)
    (Utilities|Map|Clear (Variables|Navigation|Bridge|GetPendingCompass))
    (if (Utilities|IsValid (Variables|Navigation|Bridge|GetModuleRef))
      (if (Utilities|IsValid _moduleref)
        (if (== (Widget|GetOwningPlayer _moduleref) _asplayer_controller)
          (Default|RemoveAllCompassMarkers (Variables|Navigation|Bridge|GetModuleRef)))))))

(fn AddorUpdateWorldMarker
  (params (Marker_Object :type Object%20Object%20Reference) (MarkerInfo :type S%20World%20Marker%20Info%20H%20Structure))
  (bind _moduleref (Variables|Navigation|Bridge|GetModuleRef))
  (bind _asplayer_controller (Utilities|Casting|CastToPlayerController (Components|GetOwner)))
  (if (Pawn|IsLocalController _asplayer_controller)
    (if (and (Utilities|IsValid Marker_Object) (or (Class|GameplayStatics|ObjectIsA Marker_Object "/Script/Engine.Actor") (Class|GameplayStatics|ObjectIsA Marker_Object "/Script/Engine.SceneComponent")))
      (if (and (Variables|Navigation|Bridge|GetbReady) (Utilities|IsValid (Variables|Navigation|Bridge|GetModuleRef)))
        (if (Utilities|IsValid _moduleref)
          (if (== (Widget|GetOwningPlayer _moduleref) _asplayer_controller)
            (Utilities|Map|Remove (Variables|Navigation|Bridge|GetPendingWorld) Marker_Object)
            (Default|AddorUpdateWorldMarker (Variables|Navigation|Bridge|GetModuleRef) Marker_Object MarkerInfo)))
        (elif (or (Utilities|Map|Contains (Variables|Navigation|Bridge|GetPendingWorld) Marker_Object) (< (Utilities|Map|Length (Variables|Navigation|Bridge|GetPendingWorld)) 128))
          (Utilities|Map|Add (Variables|Navigation|Bridge|GetPendingWorld) Marker_Object MarkerInfo)
          (else
            (Variables|Navigation|Bridge|SetbPendingOverflow true)))))))

(fn RemoveWorldMarker
  (params (Marker_Object :type Object%20Object%20Reference))
  (bind _moduleref (Variables|Navigation|Bridge|GetModuleRef))
  (bind _asplayer_controller (Utilities|Casting|CastToPlayerController (Components|GetOwner)))
  (if (Pawn|IsLocalController _asplayer_controller)
    (Utilities|Map|Remove (Variables|Navigation|Bridge|GetPendingWorld) Marker_Object)
    (if (Utilities|IsValid (Variables|Navigation|Bridge|GetModuleRef))
      (if (Utilities|IsValid _moduleref)
        (if (== (Widget|GetOwningPlayer _moduleref) _asplayer_controller)
          (Default|RemoveWorldMarker (Variables|Navigation|Bridge|GetModuleRef) Marker_Object))))))

(fn RemoveAllWorldMarkers
  (bind _moduleref (Variables|Navigation|Bridge|GetModuleRef))
  (bind _asplayer_controller (Utilities|Casting|CastToPlayerController (Components|GetOwner)))
  (if (Pawn|IsLocalController _asplayer_controller)
    (Utilities|Map|Clear (Variables|Navigation|Bridge|GetPendingWorld))
    (if (Utilities|IsValid (Variables|Navigation|Bridge|GetModuleRef))
      (if (Utilities|IsValid _moduleref)
        (if (== (Widget|GetOwningPlayer _moduleref) _asplayer_controller)
          (Default|RemoveAllWorldMarkers (Variables|Navigation|Bridge|GetModuleRef)))))))

(fn ShowCompass
  (bind _moduleref (Variables|Navigation|Bridge|GetModuleRef))
  (bind _asplayer_controller (Utilities|Casting|CastToPlayerController (Components|GetOwner)))
  (if (Pawn|IsLocalController _asplayer_controller)
    (Variables|Navigation|Bridge|SetbCompassVisible true)
    (Variables|Navigation|Bridge|SetbPendingVisibility true)
    (if (and (Variables|Navigation|Bridge|GetbReady) (Utilities|IsValid (Variables|Navigation|Bridge|GetModuleRef)))
      (if (Utilities|IsValid _moduleref)
        (if (== (Widget|GetOwningPlayer _moduleref) _asplayer_controller)
          (Variables|Navigation|Bridge|SetbPendingVisibility false)
          (Default|ShowCompass (Variables|Navigation|Bridge|GetModuleRef)))))))

(fn HideCompass
  (bind _moduleref (Variables|Navigation|Bridge|GetModuleRef))
  (bind _asplayer_controller (Utilities|Casting|CastToPlayerController (Components|GetOwner)))
  (if (Pawn|IsLocalController _asplayer_controller)
    (Variables|Navigation|Bridge|SetbCompassVisible false)
    (Variables|Navigation|Bridge|SetbPendingVisibility true)
    (if (and (Variables|Navigation|Bridge|GetbReady) (Utilities|IsValid (Variables|Navigation|Bridge|GetModuleRef)))
      (if (Utilities|IsValid _moduleref)
        (if (== (Widget|GetOwningPlayer _moduleref) _asplayer_controller)
          (Variables|Navigation|Bridge|SetbPendingVisibility false)
          (Default|HideCompass (Variables|Navigation|Bridge|GetModuleRef)))))))

(fn AttachModule
  (params (Module :type WBP%20AZ%20Compass%20Module%20Object%20Reference))
  (bind _asplayer_controller (Utilities|Casting|CastToPlayerController (Components|GetOwner)))
  (if (Pawn|IsLocalController _asplayer_controller)
    (if (Utilities|IsValid Module)
      (if (== (Widget|GetOwningPlayer Module) _asplayer_controller)
        (Variables|Navigation|Bridge|SetbAttached true)
        (if (not (== Module (Variables|Navigation|Bridge|GetModuleRef)))
          (Variables|Navigation|Bridge|SetbReady false)
          (Variables|Navigation|Bridge|SetModuleRef Module))))))

(fn MarkReady
  (params (Module :type WBP%20AZ%20Compass%20Module%20Object%20Reference))
  (if (Variables|Navigation|Bridge|GetbAttached)
    (bind _asplayer_controller (Utilities|Casting|CastToPlayerController (Components|GetOwner)))
    (if (Pawn|IsLocalController _asplayer_controller)
      (if (== Module (Variables|Navigation|Bridge|GetModuleRef))
        (if (Utilities|IsValid Module)
          (if (== (Widget|GetOwningPlayer Module) _asplayer_controller)
            (if (not (Variables|Navigation|Bridge|GetbReady))
              (Variables|Navigation|Bridge|SetbReady true)
              (bind _keys (Utilities|Map|Keys (Variables|Navigation|Bridge|GetPendingCompass)))
              (for _array_element _keys
                (if (== Module (Variables|Navigation|Bridge|GetModuleRef))
                  (if (Utilities|IsValid Module)
                    (if (== (Widget|GetOwningPlayer Module) _asplayer_controller)
                      (if (.ReturnValue (Utilities|Map|Find (Variables|Navigation|Bridge|GetPendingCompass) _array_element))
                        (LocalVariables|SetReplayCompassInfo (.Value (Utilities|Map|Find (Variables|Navigation|Bridge|GetPendingCompass) _array_element)))
                        (Utilities|Map|Remove (Variables|Navigation|Bridge|GetPendingCompass) _array_element)
                        (CallFunction|AddorUpdateCompassMarker _array_element (LocalVariables|GetReplayCompassInfo)))))))
              (bind _keys_2 (Utilities|Map|Keys (Variables|Navigation|Bridge|GetPendingWorld)))
              (for _array_element_2 _keys_2
                (if (== Module (Variables|Navigation|Bridge|GetModuleRef))
                  (if (Utilities|IsValid Module)
                    (if (== (Widget|GetOwningPlayer Module) _asplayer_controller)
                      (if (.ReturnValue (Utilities|Map|Find (Variables|Navigation|Bridge|GetPendingWorld) _array_element_2))
                        (LocalVariables|SetReplayWorldInfo (.Value (Utilities|Map|Find (Variables|Navigation|Bridge|GetPendingWorld) _array_element_2)))
                        (Utilities|Map|Remove (Variables|Navigation|Bridge|GetPendingWorld) _array_element_2)
                        (CallFunction|AddorUpdateWorldMarker _array_element_2 (LocalVariables|GetReplayWorldInfo)))))))
              (if (== Module (Variables|Navigation|Bridge|GetModuleRef))
                (if (Utilities|IsValid Module)
                  (if (== (Widget|GetOwningPlayer Module) _asplayer_controller)
                    (if (Variables|Navigation|Bridge|GetbPendingVisibility)
                      (Variables|Navigation|Bridge|SetbPendingVisibility false)
                      (if (Variables|Navigation|Bridge|GetbCompassVisible)
                        (Default|ShowCompass (Variables|Navigation|Bridge|GetModuleRef))
                        (else
                          (Default|HideCompass (Variables|Navigation|Bridge|GetModuleRef)))))))))))))))

(fn DetachModule
  (params (Module :type WBP%20AZ%20Compass%20Module%20Object%20Reference))
  (bind _asplayer_controller (Utilities|Casting|CastToPlayerController (Components|GetOwner)))
  (if (Pawn|IsLocalController _asplayer_controller)
    (if (== Module (Variables|Navigation|Bridge|GetModuleRef))
      (Variables|Navigation|Bridge|SetbReady false)
      (Variables|Navigation|Bridge|SetbAttached false))))