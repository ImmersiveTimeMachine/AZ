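; Gameplay Ability that makes the hero sprint while the input is held.
; On activation it applies GE_Sprint to the owner and waits for input release, then ends the ability.
; Ending the ability removes all stacks of GE_Sprint from the owner's Ability System Component.
; Disconnected nodes that cast to BP_CMC_Hero and set MaxWalkSpeed directly remain in the graph but never run.
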(event Ability|EventActivateAbility
  (Ability|ApplyGameplayEffectToOwner "/Game/AZ/Blueprints/AbilitySystem/Hero/Effects/GE_Sprint.GE_Sprint_C")
  (Ability|Tasks|WaitInputRelease true
    (:OnRelease
      (Ability|EndAbility))))

(event Ability|EventOnEndAbility
  (params (bWasCancelled :type Boolean))
  (GameplayEffects|RemoveActiveGameplayEffectbySourceEffect (Ability|GetAbilitySystemComponentfromActorInfo) "/Game/AZ/Blueprints/AbilitySystem/Hero/Effects/GE_Sprint.GE_Sprint_C" 0 -1))