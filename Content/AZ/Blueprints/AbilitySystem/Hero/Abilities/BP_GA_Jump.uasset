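; Gameplay ability for the hero's jump, adding a momentum boost rather than calling the character jump.
; On activation it waits for the unarmed EndJumping animation gameplay event to end itself.
; If the hero has the Walking tag, it adds a velocity-change impulse scaled from current movement velocity.
; The CharacterJumpStart/Stop with input-release path and a montage task are left unconnected.
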(event Ability|EventActivateAbility
  (bind _asaz_bp_hero (Utilities|Casting|CastToAZ_BP_Hero (Ability|GetAvatarActorfromActorInfo)))
  (Utilities|FlowControl|Sequence
    (:then_0
      (Ability|Async|WaitGameplayEventToActor _asaz_bp_hero "(TagName=\"Animation.State.Unarmed.EndJumping\")"
        (:EventReceived
          (Ability|EndAbility))))
    (:then_1
      (if (GameplayTags|HasMatchingGameplayTag (Class|AZCharacterBase|GetASC _asaz_bp_hero) "(TagName=\"Movement.Walking\")")
        (Physics|AddImpulse (Variables|/Script/Engine.Character|GetCharacterMovement _asaz_bp_hero) (* (Variables|/Script/Engine.MovementComponent|GetVelocity (Variables|/Script/Engine.Character|GetCharacterMovement _asaz_bp_hero)) (Variables|Default|GetJumpImpuls)) true)))))

(event Ability|EventOnEndAbility
  (params (bWasCancelled :type Boolean)))