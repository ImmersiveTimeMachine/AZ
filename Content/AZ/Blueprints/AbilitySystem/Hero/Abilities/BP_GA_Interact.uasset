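; Gameplay ability that performs the hero's interact action.
; On activation it casts the avatar to AZ_BP_Hero, calls PrimaryInteract on its BP_AZ_PlayerController, then ends after a short delay.
; The graph also holds several disconnected drafts that never run, covering weapon and item pickup, back-socket attachment and target-data rifle detection.
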(event Ability|EventActivateAbility
  (bind _asaz_bp_hero (Utilities|Casting|CastToAZ_BP_Hero (Ability|GetAvatarActorfromActorInfo)))
  (bind _asbp_az_player_controller (Utilities|Casting|CastToBP_AZ_PlayerController (Pawn|GetController _asaz_bp_hero)))
  (Class|AZPlayerController|PrimaryInteract _asbp_az_player_controller)
  (Utilities|FlowControl|Delay 2.0)
  (Ability|EndAbility))

(event Ability|EventOnEndAbility
  (params (bWasCancelled :type Boolean)))