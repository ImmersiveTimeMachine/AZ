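; Hero gameplay ability that toggles the CommonUI inventory menu.
; On activation it casts the avatar's owner to the AZ player controller, calls its toggle function, then ends immediately.
; The graph also holds disconnected logic that never runs: weapon and item pickup, attaching a spawned item to a back socket, an older menu toggle, and a target-data rifle detection test.
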(event Ability|EventActivateAbility
  (bind _asbp_az_player_controller (Utilities|Casting|CastToBP_AZ_PlayerController (Components|GetOwner (Ability|GetAvatarActorfromActorInfo)))
    (:then
      (Class|AZPlayerController|ToggleCommonUIInventoryMenu _asbp_az_player_controller))
    (:CastFailed
      _))
  (Ability|EndAbility))

(event Ability|EventOnEndAbility
  (params (bWasCancelled :type Boolean)))